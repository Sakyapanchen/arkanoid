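; BP_FieldBorder is a field boundary actor that turns back projectiles affecting it.
; On BeginPlay it resizes its bounds box in X and Y from BorderExtent, keeping Z, then generates a colored procedural border mesh from that box.
; AffectionRequest accepts only BP_Projectile, clearing its buff stack and rotating it, and returns whether the cast succeeded.
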(event EventBeginPlay
  (bind _borderextent (Variables|Settings|GetBorderExtent))
  (bind (_x _y) (Math|Vector|BreakVector _borderextent))
  (Components|Box|SetBoxExtent (Variables|Default|GetBorderBounds) (Math|Vector|MakeVector _x _y (.Z (Math|Vector|BreakVector (Variables|/Script/Engine.BoxComponent|GetBoxExtent (Variables|Default|GetBorderBounds))))) true)
  (Default|GenerateProceduralMesh (Variables|Default|GetBorderMesh) (Variables|Default|GetBorderBounds) "(R=0.213147,G=0.000000,B=0.640625,A=1.000000)"))

(fn ConstructionScript)

(fn AffectionRequest
  (params (Hit :type Hit%20Result%20Structure) (Projectile :type Actor%20Object%20Reference))
  (bind _asbp_projectile (Utilities|Casting|CastToBP_Projectile Projectile)
    (:then
      (LocalVariables|SetL_Projectile _asbp_projectile)
      (Default|DiscardBaffStack (LocalVariables|GetL_Projectile))
      (Default|RotateProjectile (LocalVariables|GetL_Projectile))
      (return true))
    (:CastFailed
      (return false))))