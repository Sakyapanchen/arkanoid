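; Arkanoid ball projectile, sized from the GameMode's brick height and launched by detaching at a random ±45 degree yaw.
; Each tick it sweeps forward at a speed that rises with level.
; Hits are forwarded to the struck actor as an AffectionRequest message, while RotateProjectile mirrors the heading on the impact normal's axes.
; A stackable buff counter switches the dynamic material's color until discarded to zero.
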(event OnComponentHit(Sphere)
  (params (HitComponent :type Primitive%20Component%20Object%20Reference) (OtherActor :type Actor%20Object%20Reference) (OtherComp :type Primitive%20Component%20Object%20Reference) (NormalImpulse :type Vector :default "0, 0, 0") (Hit :type Hit%20Result%20Structure%20%28by%20ref%29))
  (CallFunction|HitHandler Hit))

(event EventBeginPlay
  (CallFunction|SetStartParams))

(event EventTick
  (params (DeltaSeconds :type Float%20%28single-precision%29))
  (|CallParentFunction DeltaSeconds)
  (CallFunction|ProjectileMovement))

(fn ConstructionScript)

(fn SetStartParams
  (Collision|SetCollisionEnabled (Variables|Default|GetSphere) "NoCollision")
  (Variables|References|SetGameMode (CallFunction|GetArkanoidGameMode self))
  (Transformation|SetRelativeScale3D (Variables|Default|GetProjectileMesh) (Math|Vector|MakeVector (/ (/ (Math|Conversions|ToFloat(Integer) (Variables|/Script/Arkanoid.ArkanoidGameMode|GetBrickHeight (Variables|References|GetGameMode))) 2.0) (Variables|/Script/Engine.SphereComponent|GetSphereRadius (Variables|Default|GetSphere))) (/ (/ (Math|Conversions|ToFloat(Integer) (Variables|/Script/Arkanoid.ArkanoidGameMode|GetBrickHeight (Variables|References|GetGameMode))) 2.0) (Variables|/Script/Engine.SphereComponent|GetSphereRadius (Variables|Default|GetSphere))) (/ (/ (Math|Conversions|ToFloat(Integer) (Variables|/Script/Arkanoid.ArkanoidGameMode|GetBrickHeight (Variables|References|GetGameMode))) 2.0) (Variables|/Script/Engine.SphereComponent|GetSphereRadius (Variables|Default|GetSphere)))))
  (Components|Sphere|SetSphereRadius (Variables|Default|GetSphere) (/ (Math|Conversions|ToFloat(Integer) (Variables|/Script/Arkanoid.ArkanoidGameMode|GetBrickHeight (Variables|References|GetGameMode))) 2.0) true)
  (bind _returnvalue (Rendering|Material|CreateDynamicMaterialInstance (Variables|Default|GetProjectileMesh) 0 (Rendering|Material|GetMaterial (Variables|Default|GetProjectileMesh) 0) "None" :!class /Script/Engine.PrimitiveComponent))
  (Variables|References|SetProjectileDMI _returnvalue)
  (Rendering|Material|SetMaterial (Variables|Default|GetProjectileMesh) 0 (Variables|References|GetProjectileDMI))
  (Rendering|Material|SetVectorParameterValue (Variables|References|GetProjectileDMI) "Color" (Variables|/Script/Arkanoid.ArkanoidGameMode|GetProjectileDefaultColor (Variables|References|GetGameMode)) :!class /Script/Engine.MaterialInstanceDynamic))

(fn StartMovement
  (Collision|SetCollisionEnabled (Variables|Default|GetSphere) "QueryAndPhysics")
  (Transformation|DetachFromActor self "KeepWorld" "KeepWorld" "KeepWorld")
  (Class|Actor|AddActorWorldRotation self (Math|Rotator|MakeRotator 0.0 0.0 (select (Math|Random|RandomBool) 45.0 -45.0)))
  (Variables|Private|SetMovementAllow true))

(fn HitHandler
  (params (Hit :type Hit%20Result%20Structure))
  (Variables|Default|SetCurrentHit Hit)
  (Class|Affector|AffectionRequest(Message) (.HitActor (Collision|BreakHitResult (Variables|Default|GetCurrentHit))) (Variables|Default|GetCurrentHit) self))

(fn ProjectileMovement
  (if (Variables|Private|GetMovementAllow)
    (Transformation|AddActorLocalOffset (Math|Vector|MakeVector (* (+ (Variables|/Script/Arkanoid.ArkanoidGameMode|GetProjectileStartSpeed (Variables|References|GetGameMode)) (* (- (Variables|/Script/Arkanoid.ArkanoidGameMode|GetCurrentLevel (Variables|References|GetGameMode)) 1) (Variables|/Script/Arkanoid.ArkanoidGameMode|GetProjectileSpeedIncrease (Variables|References|GetGameMode)))) (Utilities|Time|GetWorldDeltaSeconds)) 0.0 0.0) true false)))

(fn UpdateBaff
  (Variables|Private|SetRemainBaffTime (+ (Variables|Private|GetRemainBaffTime) (Variables|/Script/Arkanoid.ArkanoidGameMode|GetLegendaryBrickBaffTime (Variables|References|GetGameMode))))
  (Rendering|Material|SetVectorParameterValue (Variables|References|GetProjectileDMI) "Color" (Variables|/Script/Arkanoid.ArkanoidGameMode|GetProjectileBaffedColor (Variables|References|GetGameMode)) :!class /Script/Engine.MaterialInstanceDynamic))

(fn DiscardBaffStack
  (if (> (Variables|Private|GetRemainBaffTime) 0)
    (Math|Integer|DecrementInt (Variables|Private|GetRemainBaffTime)
      (:%20%20
        (if (<= (Variables|Private|GetRemainBaffTime) 0)
          (Rendering|Material|SetVectorParameterValue (Variables|References|GetProjectileDMI) "Color" (Variables|/Script/Arkanoid.ArkanoidGameMode|GetProjectileDefaultColor (Variables|References|GetGameMode)) :!class /Script/Engine.MaterialInstanceDynamic))))))

(fn GetReaminBaffTime
  (return (Variables|Private|GetRemainBaffTime)))

(fn RotateProjectile
  (LocalVariables|SetL_ImpactNormal (.ImpactNormal (Collision|BreakHitResult (Variables|Default|GetCurrentHit))))
  (LocalVariables|SetL_NewForwardVector (Transformation|GetActorForwardVector))
  (Utilities|FlowControl|Sequence
    (:then_0
      (if (!= (.X (Math|Vector|BreakVector (LocalVariables|GetL_ImpactNormal))) 0.0)
        (LocalVariables|SetL_NewForwardVector (Math|Vector|MakeVector (* -1.0 (.X (Math|Vector|BreakVector (LocalVariables|GetL_NewForwardVector)))) (.Y (Math|Vector|BreakVector (LocalVariables|GetL_NewForwardVector))) (.Z (Math|Vector|BreakVector (LocalVariables|GetL_NewForwardVector)))))))
    (:then_1
      (if (!= (.Y (Math|Vector|BreakVector (LocalVariables|GetL_ImpactNormal))) 0.0)
        (LocalVariables|SetL_NewForwardVector (Math|Vector|MakeVector (.X (Math|Vector|BreakVector (LocalVariables|GetL_NewForwardVector))) (* -1.0 (.Y (Math|Vector|BreakVector (LocalVariables|GetL_NewForwardVector)))) (.Z (Math|Vector|BreakVector (LocalVariables|GetL_NewForwardVector)))))))
    (:then_2
      (Transformation|SetActorRotation (Math|Rotator|MakeRotfromX (LocalVariables|GetL_NewForwardVector)) true))))