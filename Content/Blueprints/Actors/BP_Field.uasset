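; BP_Field is the Arkanoid playfield actor that acts as the view target and builds the brick layout at BeginPlay.
; It sizes FieldBounds from GameMode brick and field dimensions, then generates the field's procedural mesh from that box.
; It spawns a grid of randomly chosen common, rare or legendary bricks, alternating columns outward from the center line.
; Tick's UpdateCamera only prints a debug corner position; its ortho-width fitting is disconnected.
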(event EventBeginPlay
  (|CallParentFunction)
  (CallFunction|SetStartParams)
  (Default|GenerateProceduralMesh (Variables|Default|GetFieldMesh) (Variables|Default|GetFieldBounds) "(R=0.019382,G=0.019382,B=0.019382,A=1.000000)")
  (CallFunction|GenerateBricks))

(event EventTick
  (params (DeltaSeconds :type Float%20%28single-precision%29))
  (|CallParentFunction DeltaSeconds)
  (CallFunction|UpdateCamera))

(fn ConstructionScript)

(fn SetStartParams
  (Utilities|FlowControl|Sequence
    (:then_0
      (Variables|References|SetGameMode (CallFunction|GetArkanoidGameMode self))
      (Game|Player|SetViewTargetwithBlend (Game|GetPlayerController 0) self 0.0 "VTBlend_Linear" 0.0 false))
    (:then_1
      (Components|Box|SetBoxExtent (Variables|Default|GetFieldBounds) (Math|Vector|MakeVector (/ (Math|Conversions|ToFloat(Integer) (* (Variables|/Script/Arkanoid.ArkanoidGameMode|GetBrickHeight (Variables|References|GetGameMode)) (Variables|/Script/Arkanoid.ArkanoidGameMode|GetFieldHeight (Variables|References|GetGameMode)))) 2.0) (/ (Math|Conversions|ToFloat(Integer) (* (Variables|/Script/Arkanoid.ArkanoidGameMode|GetBrickWidth (Variables|References|GetGameMode)) (Variables|/Script/Arkanoid.ArkanoidGameMode|GetFieldWidth (Variables|References|GetGameMode)))) 2.0) (.Z (Math|Vector|BreakVector (Variables|/Script/Engine.BoxComponent|GetBoxExtent (Variables|Default|GetFieldBounds))))) false))))

(fn GenerateBricks
  (Utilities|Array|Clear (Variables|References|GetBricks))
  (for _index (range 1 (Variables|/Script/Arkanoid.ArkanoidGameMode|GetBrickRowsCount (Variables|References|GetGameMode)))
    (LocalVariables|SetL_CurrentRow _index)
    (for _index_2 (range 1 (Variables|/Script/Arkanoid.ArkanoidGameMode|GetBrickColumnsCount (Variables|References|GetGameMode)))
      (LocalVariables|SetL_CurrentColumn _index_2)
      (bind _returnvalue (Game|SpawnActorfromClass (CallFunction|GetBrickClass) (CallFunction|CalculateBrickSpawnTransform (LocalVariables|GetL_CurrentRow) (LocalVariables|GetL_CurrentColumn)) "AdjustIfPossibleButDontSpawnIfColliding" self 0))
      (Utilities|Array|Add (Variables|References|GetBricks) _returnvalue))))

(fn UpdateCamera
  (bind _returnvalue (Transformation|GetActorLocation))
  (bind _fieldbounds (Variables|Default|GetFieldBounds))
  (bind (_x _y) (Math|Vector|BreakVector _returnvalue))
  (bind _boxextent (Variables|/Script/Engine.BoxComponent|GetBoxExtent _fieldbounds))
  (bind (_x_2 _y_2) (Math|Vector|BreakVector _boxextent))
  (Development|PrintString (Utilities|String|ToString(Vector) (Math|Vector|MakeVector (+ _x_2 _x) (+ _y_2 _y) 0.0)) true false "(R=1.000000,G=0.000000,B=0.997643,A=1.000000)" 0.0))

(fn GetBrickClass
  (return (Utilities|Select :Index (Math|Random|RandomIntegerinRange 0 2) :Option%200 "/Game/Blueprints/Actors/Bricks/BP_CommonBrick.BP_CommonBrick_C" :Option%201 "/Game/Blueprints/Actors/Bricks/BP_RareBrick.BP_RareBrick_C" :Option%202 "/Game/Blueprints/Actors/Bricks/BP_LegendaryBrick.BP_LegendaryBrick_C")))

(fn CalculateBrickSpawnTransform
  (params (Row :type Integer) (Column :type Integer))
  (LocalVariables|SetL_CurrentRow Row)
  (LocalVariables|SetL_CurrentColumn Column)
  (Utilities|FlowControl|Sequence
    (:then_0
      (bind _output_get (LocalVariables|SetL_SpawnLocation (Transformation|GetActorLocation)))
      (LocalVariables|SetL_SpawnLocation (Math|Vector|MakeVector (+ (- (* (Math|Conversions|ToFloat(Integer) (LocalVariables|GetL_CurrentRow)) (Math|Conversions|ToFloat(Integer) (Variables|/Script/Arkanoid.ArkanoidGameMode|GetBrickHeight (Variables|References|GetGameMode)))) (/ (Math|Conversions|ToFloat(Integer) (Variables|/Script/Arkanoid.ArkanoidGameMode|GetBrickHeight (Variables|References|GetGameMode))) 2.0)) (.X (Math|Vector|BreakVector _output_get))) (.Y (Math|Vector|BreakVector _output_get)) (+ (.Z (Math|Vector|BreakVector _output_get)) 1e+02))))
    (:then_1
      (Utilities|FlowControl|Sequence
        (:then_0
          (if (> (Math|Integer|%(Integer) (LocalVariables|GetL_CurrentColumn) 2) 0)
            (LocalVariables|SetL_SpawnYDisplacement (* (- (* (/ (Math|Conversions|ToFloat(Integer) (+ (LocalVariables|GetL_CurrentColumn) 1)) 2.0) (Math|Conversions|ToFloat(Integer) (Variables|/Script/Arkanoid.ArkanoidGameMode|GetBrickWidth (Variables|References|GetGameMode)))) (/ (Math|Conversions|ToFloat(Integer) (Variables|/Script/Arkanoid.ArkanoidGameMode|GetBrickWidth (Variables|References|GetGameMode))) 2.0)) -1.0))
            (else
              (LocalVariables|SetL_SpawnYDisplacement (- (* (/ (Math|Conversions|ToFloat(Integer) (LocalVariables|GetL_CurrentColumn)) 2.0) (Math|Conversions|ToFloat(Integer) (Variables|/Script/Arkanoid.ArkanoidGameMode|GetBrickWidth (Variables|References|GetGameMode)))) (/ (Math|Conversions|ToFloat(Integer) (Variables|/Script/Arkanoid.ArkanoidGameMode|GetBrickWidth (Variables|References|GetGameMode))) 2.0))))))
        (:then_1
          (LocalVariables|SetL_SpawnLocation (Math|Vector|MakeVector (.X (Math|Vector|BreakVector (LocalVariables|GetL_SpawnLocation))) (+ (.Y (Math|Vector|BreakVector (LocalVariables|GetL_SpawnLocation))) (LocalVariables|GetL_SpawnYDisplacement)) (.Z (Math|Vector|BreakVector (LocalVariables|GetL_SpawnLocation))))))))
    (:then_2
      (return (Math|Transform|MakeTransform (LocalVariables|GetL_SpawnLocation))))))