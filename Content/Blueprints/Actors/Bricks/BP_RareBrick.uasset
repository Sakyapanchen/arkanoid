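; BP_RareBrick is a rare brick variant that takes its color from the GameMode's RareBrick settings.
; When hit by a BP_Projectile, it asks the GameMode to destroy its neighboring bricks, then itself.
; A projectile with remaining buff time discards a buff stack instead of rotating; an unbuffed one rotates.
; Other projectile types leave the brick untouched and the request returns false.
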(fn ConstructionScript
  (|CallParentFunction))

(fn GetBrickColor
  (bind _gamemode (Variables|Default|GetGameMode)
    (:then
      (return (Utilities|Struct|BreakBrickData (Variables|/Script/Arkanoid.ArkanoidGameMode|GetRareBrick _gamemode))))
    (:else)))

(fn AffectionRequest
  (params (Hit :type Hit%20Result%20Structure) (Projectile :type Actor%20Object%20Reference))
  (bind _asbp_projectile (Utilities|Casting|CastToBP_Projectile Projectile)
    (:then
      (LocalVariables|SetL_Projectile _asbp_projectile)
      (Utilities|FlowControl|Sequence
        (:then_0
          (for _array_element (CallFunction|GetNeighbors)
            (Default|BrickDestroyRequest (Variables|Default|GetGameMode) _array_element)))
        (:then_1
          (if (> (Default|GetReaminBaffTime (LocalVariables|GetL_Projectile)) 0)
            (Default|DiscardBaffStack (LocalVariables|GetL_Projectile))
            (bind _success (Default|BrickDestroyRequest (Variables|Default|GetGameMode) self))
            (return _success)
            (else
              (Default|RotateProjectile (LocalVariables|GetL_Projectile))
              (bind _success_2 (Default|BrickDestroyRequest (Variables|Default|GetGameMode) self))
              (return _success_2))))))
    (:CastFailed
      (return false))))