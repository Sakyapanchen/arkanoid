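; Legendary brick variant for a brick-breaking game that triggers a buff update on the projectile that hits it.
; It runs its parent's construction script and takes its color from the GameMode's LegendaryBrick settings.
; When hit by a BP_Projectile, it calls UpdateBaff on that projectile, disables its bounds collision and returns the result of the GameMode's destroy request.
; Any other projectile type returns false.
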(fn ConstructionScript
  (|CallParentFunction))

(fn GetBrickColor
  (bind _gamemode (Variables|Default|GetGameMode)
    (:then
      (return (Utilities|Struct|BreakBrickData (Variables|/Script/Arkanoid.ArkanoidGameMode|GetLegendaryBrick _gamemode))))
    (:else)))

(fn AffectionRequest
  (params (Hit :type Hit%20Result%20Structure) (Projectile :type Actor%20Object%20Reference))
  (bind _asbp_projectile (Utilities|Casting|CastToBP_Projectile Projectile)
    (:then
      (LocalVariables|SetL_Projectile _asbp_projectile)
      (Default|UpdateBaff (LocalVariables|GetL_Projectile))
      (Collision|SetCollisionEnabled (Variables|Default|GetBrickBounds) "NoCollision")
      (bind _success (Default|BrickDestroyRequest (Variables|Default|GetGameMode) self))
      (return _success))
    (:CastFailed
      (return false))))