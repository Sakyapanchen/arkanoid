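; BP_CommonBrick is the standard brick actor in a projectile-and-brick game, taking its color from the GameMode's CommonBrick settings.
; AffectionRequest handles a projectile hit by increasing the score, then asking the GameMode to destroy the brick and returning that result.
; A projectile with remaining buff time has a buff stack discarded instead of being rotated, and non-BP_Projectile callers get false.
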(event EventBeginPlay
  (|CallParentFunction) ; This node is disabled and will not be called.\nDrag off pins to build functionality.
)

(event Collision|EventActorBeginOverlap
  (params (OtherActor :type Actor%20Object%20Reference)))

(event EventTick
  (params (DeltaSeconds :type Float%20%28single-precision%29)))

(fn ConstructionScript
  (|CallParentFunction))

(fn GetBrickColor
  (bind _gamemode (Variables|Default|GetGameMode)
    (:then
      (return (Utilities|Struct|BreakBrickData (Variables|/Script/Arkanoid.ArkanoidGameMode|GetCommonBrick _gamemode))))
    (:else)))

(fn AffectionRequest
  (params (Hit :type Hit%20Result%20Structure) (Projectile :type Actor%20Object%20Reference))
  (LocalVariables|SetL_Hit Hit)
  (bind _asbp_projectile (Utilities|Casting|CastToBP_Projectile Projectile)
    (:then
      (LocalVariables|SetL_Projectile _asbp_projectile)
      (Default|IncreaseCurrentScore (Variables|Default|GetGameMode))
      (if (> (Default|GetReaminBaffTime (LocalVariables|GetL_Projectile)) 0)
        (Default|DiscardBaffStack (LocalVariables|GetL_Projectile))
        (bind _success (Default|BrickDestroyRequest (Variables|Default|GetGameMode) self))
        (return _success)
        (else
          (Default|RotateProjectile (LocalVariables|GetL_Projectile))
          (bind _success_2 (Default|BrickDestroyRequest (Variables|Default|GetGameMode) self))
          (return _success_2))))
    (:CastFailed
      (return false))))