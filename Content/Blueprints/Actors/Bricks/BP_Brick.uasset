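; BP_Brick is an Arkanoid brick actor that sizes its bounds from the game mode's brick dimensions on BeginPlay.
; It then generates a procedural mesh from those bounds in the color from GetBrickColor, a fixed red.
; GetNeighbors finds adjacent bricks with four Visibility line traces along the X and Y axes.
; AffectionRequest takes a hit and projectile but simply returns false here.
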(event EventBeginPlay
  (|CallParentFunction)
  (CallFunction|SetStartParams)
  (Default|GenerateProceduralMesh (Variables|Default|GetBrickMesh) (Variables|Default|GetBrickBounds) (CallFunction|GetBrickColor)))

(fn ConstructionScript)

(fn GetBrickColor
  (return "(R=1.000000,G=0.000000,B=0.114047,A=1.000000)"))

(fn SetStartParams
  (Variables|References|SetGameMode (CallFunction|GetArkanoidGameMode self))
  (Components|Box|SetBoxExtent (Variables|Default|GetBrickBounds) (Math|Vector|MakeVector (/ (Math|Conversions|ToFloat(Integer) (Variables|/Script/Arkanoid.ArkanoidGameMode|GetBrickHeight (Variables|References|GetGameMode))) 2.0) (/ (Math|Conversions|ToFloat(Integer) (Variables|/Script/Arkanoid.ArkanoidGameMode|GetBrickWidth (Variables|References|GetGameMode))) 2.0) (.Z (Math|Vector|BreakVector (Variables|/Script/Engine.BoxComponent|GetBoxExtent (Variables|Default|GetBrickBounds))))) true)
  (Transformation|SetRelativeLocation (Variables|Default|GetBrickMesh) (Math|Vector|MakeVector 0.0 0.0 (.Z (Math|Vector|BreakVector (Variables|/Script/Engine.BoxComponent|GetBoxExtent (Variables|Default|GetBrickBounds))))) false true))

(fn GetNeighbors
  (Utilities|FlowControl|Sequence
    (:then_0
      (for _index (range 0 3)
        (LocalVariables|SetL_Index _index)
        (LocalVariables|SetL_TraceEnd (Utilities|Select :Index (LocalVariables|GetL_Index) :Option%200 (+ (Transformation|GetActorLocation) (Math|Vector|MakeVector (* (.X (Math|Vector|BreakVector (Variables|/Script/Engine.BoxComponent|GetBoxExtent (Variables|Default|GetBrickBounds)))) 2.0) 0.0 0.0)) :Option%201 (+ (Transformation|GetActorLocation) (Math|Vector|MakeVector 0.0 (* (.Y (Math|Vector|BreakVector (Variables|/Script/Engine.BoxComponent|GetBoxExtent (Variables|Default|GetBrickBounds)))) 2.0) 0.0)) :Option%202 (+ (Transformation|GetActorLocation) (Math|Vector|MakeVector (* (.X (Math|Vector|BreakVector (Variables|/Script/Engine.BoxComponent|GetBoxExtent (Variables|Default|GetBrickBounds)))) -2.0) 0.0 0.0)) :Option%203 (+ (Transformation|GetActorLocation) (Math|Vector|MakeVector 0.0 (* (.Y (Math|Vector|BreakVector (Variables|/Script/Engine.BoxComponent|GetBoxExtent (Variables|Default|GetBrickBounds)))) -2.0) 0.0))))
        (bind (_outhit _returnvalue) (Collision|LineTraceByChannel (Transformation|GetActorLocation) (LocalVariables|GetL_TraceEnd) "TraceTypeQuery1" true 0 "None"))
        (if _returnvalue
          (bind _asbp_brick (Utilities|Casting|CastToBP_Brick (.HitActor (Collision|BreakHitResult _outhit))))
          (Utilities|Array|Add (LocalVariables|GetL_Neighbors) _asbp_brick))))
    (:then_1
      (return (LocalVariables|GetL_Neighbors)))))

(fn AffectionRequest
  (params (Hit :type Hit%20Result%20Structure) (Projectile :type Actor%20Object%20Reference))
  (return false))