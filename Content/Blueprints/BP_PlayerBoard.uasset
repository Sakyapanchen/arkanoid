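; BP_PlayerBoard is the player's Arkanoid paddle, moved sideways by mouse with a swept offset and launching the ball on left click.
; On BeginPlay it sizes its bounds from the game mode's brick and board settings, builds a procedural mesh and spawns an attached projectile.
; ProjectileGone destroys the ball, decrements hit points through the game mode and spawns a replacement.
; AffectionRequest clears a hitting projectile's buff stack and rotates it.
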(event EventBeginPlay
  (CallFunction|SetStartParams)
  (Default|GenerateProceduralMesh (Variables|Default|GetPlayerProceduralMesh) (Variables|Default|GetPlayerBounds) "(R=0.505208,G=0.366923,B=0.123027,A=1.000000)")
  (CallFunction|SpawnProjectile))

(event Input|MouseEvents|MouseX
  (params (AxisValue :type Float%20%28single-precision%29))
  (CallFunction|BoardLeftRightMove AxisValue))

(event Input|MouseEvents|LeftMouseButton
  (params (Key :type Key%20Structure))
  (:Pressed
    (CallFunction|Fire)))

(fn ConstructionScript)

(fn SetStartParams
  (Variables|References|SetGameMode (CallFunction|GetArkanoidGameMode self))
  (Components|Box|SetBoxExtent (Variables|Default|GetPlayerBounds) (Math|Vector|MakeVector (/ (Math|Conversions|ToFloat(Integer) (Variables|/Script/Arkanoid.ArkanoidGameMode|GetBrickHeight (Variables|References|GetGameMode))) 2.0) (/ (Math|Conversions|ToFloat(Integer) (* (Variables|/Script/Arkanoid.ArkanoidGameMode|GetBrickWidth (Variables|References|GetGameMode)) (Variables|/Script/Arkanoid.ArkanoidGameMode|GetBoardWidth (Variables|References|GetGameMode)))) 2.0) (.Z (Math|Vector|BreakVector (Variables|/Script/Engine.BoxComponent|GetBoxExtent (Variables|Default|GetPlayerBounds))))) true)
  (Transformation|SetRelativeLocation (Variables|Default|GetPlayerProceduralMesh) (Math|Vector|MakeVector 0.0 0.0 (.Z (Math|Vector|BreakVector (Variables|/Script/Engine.BoxComponent|GetBoxExtent (Variables|Default|GetPlayerBounds))))) false true))

(fn BoardLeftRightMove
  (params (Axis :type Float%20%28single-precision%29))
  (LocalVariables|SetL_Axis Axis)
  (Transformation|AddActorLocalOffset (* (Transformation|GetActorRightVector self) (* (LocalVariables|GetL_Axis) (Variables|Settings|GetBoardSpeedMultiplier))) true false))

(fn SpawnProjectile
  (bind _returnvalue (Transformation|GetActorLocation))
  (bind (_x _y _z) (Math|Vector|BreakVector _returnvalue))
  (bind _returnvalue_2 (Game|SpawnActorfromClass "/Game/Blueprints/Actors/BP_Projectile.BP_Projectile_C" (Transformation|GetActorTransform) "AlwaysSpawn" self 0))
  (bind _output_get (Variables|References|SetCurrentProjectile _returnvalue_2))
  (Transformation|AttachComponentToComponent _output_get (Variables|Default|GetPlayerBounds) "None" "SnapToTarget" "SnapToTarget" "SnapToTarget" false)
  (Transformation|SetActorLocation (Variables|References|GetCurrentProjectile) (Math|Vector|MakeVector (+ (Math|Conversions|ToFloat(Integer) (Variables|/Script/Arkanoid.ArkanoidGameMode|GetBrickHeight (Variables|References|GetGameMode))) _x) _y _z) false true))

(fn Fire
  (bind _currentprojectile (Variables|References|GetCurrentProjectile)
    (:then
      (Default|StartMovement _currentprojectile))
    (:else)))

(fn ProjectileGone
  (Utilities|FlowControl|Sequence
    (:then_0
      (bind _currentprojectile (Variables|References|GetCurrentProjectile)
        (:then
          (Actor|DestroyActor _currentprojectile))
        (:else)))
    (:then_1
      (bind _gamemode (Variables|References|GetGameMode)
        (:then
          (Default|DecreaseHitPoints _gamemode))
        (:else)))
    (:then_2
      (CallFunction|SpawnProjectile))))

(fn AffectionRequest
  (params (Hit :type Hit%20Result%20Structure) (Projectile :type Actor%20Object%20Reference))
  (bind _asbp_projectile (Utilities|Casting|CastToBP_Projectile Projectile)
    (:then
      (LocalVariables|SetL_Projectile _asbp_projectile)
      (Default|DiscardBaffStack (LocalVariables|GetL_Projectile))
      (Default|RotateProjectile (LocalVariables|GetL_Projectile))
      (return true))
    (:CastFailed
      (return false))))