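; Game mode for an Arkanoid-style game that tracks score, max score, hit points, level and destroyed bricks.
; Starting a game or level destroys actors tagged "Gameplay" and spawns a fresh BP_Field, with FieldIsReload set during the swap.
; Dispatchers announce score, hit point and level changes, level end once destroyed bricks match the field's count, and game over, which also pauses play.
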(event EventBeginPlay
  (|CallParentFunction)
  (Game|StartNewGame))

(fn ConstructionScript)

(fn IncreaseCurrentScore
  (bind _output_get (Variables|Default|SetCurrentScore (+ (Variables|Default|GetCurrentScore) (Variables|Default|GetScoreFromBrick))))
  (Default|CallOnCurrentScoreChange self _output_get)
  (if (> (Variables|Default|GetCurrentScore) (Variables|Default|GetMaxScore))
    (bind _output_get_2 (Variables|Default|SetMaxScore (Variables|Default|GetCurrentScore)))
    (Default|CallOnMaxScoreChange self _output_get_2)))

(fn StartNewGame
  (Variables|Game|SetFieldIsReload true)
  (Game|DestroyGameplayObjects)
  (Variables|Default|SetCurrentLevel 1)
  (Variables|Default|SetCurrentHitPoints (Variables|Default|GetMaxHitPoints))
  (Default|CallOnNewLevelStarted self (Variables|Default|GetCurrentLevel))
  (bind _returnvalue (Game|SpawnActorfromClass "/Game/Blueprints/Actors/BP_Field.BP_Field_C" (Math|Transform|MakeTransform "0, 0, 0") "AlwaysSpawn" self 0))
  (Variables|References|SetField _returnvalue)
  (Variables|Game|SetFieldIsReload false))

(fn DecreaseHitPoints
  (Math|Integer|DecrementInt (Variables|Default|GetCurrentHitPoints)
    (:%20%20
      (Default|CallOnHitPointsChange self (Variables|Default|GetCurrentHitPoints))
      (if (<= (Variables|Default|GetCurrentHitPoints) 0)
        (Default|CallOnGameOver self)
        (Game|SetGamePaused true)))))

(fn BrickDestroyRequest
  (params (Brick :type BP%20Brick%20Object%20Reference))
  (Utilities|IsValid Brick
    (:Is%20Valid
      (Math|Integer|IncrementInt (Variables|Game|GetDestroyedBricksCount)
        (:%20%20
          (Actor|DestroyActor Brick)
          (if (== (Variables|Game|GetDestroyedBricksCount) (Utilities|Array|Length (Variables|/Game/Blueprints/Actors/BP_Field.BP_Field_C|GetBricks (Variables|References|GetField))))
            (Default|CallOnLevelEnd self 0 (Variables|Default|GetCurrentLevel))
            (return true)
            (else
              (return true))))))))

(fn StartNewLevel
  (Variables|Game|SetFieldIsReload true)
  (Game|DestroyGameplayObjects)
  (Math|Integer|IncrementInt (Variables|Default|GetCurrentLevel)
    (:%20%20
      (Default|CallOnNewLevelStarted self (Variables|Default|GetCurrentLevel))
      (bind _returnvalue (Game|SpawnActorfromClass "/Game/Blueprints/Actors/BP_Field.BP_Field_C" (Math|Transform|MakeTransform "0, 0, 0") "AlwaysSpawn" self 0))
      (Variables|References|SetField _returnvalue)
      (Variables|Game|SetFieldIsReload false))))

(fn DestroyGameplayObjects
  (bind _outactors (Actor|GetAllActorswithTag "Gameplay"))
  (for _array_element _outactors
    (Utilities|IsValid _array_element
      (:Is%20Valid
        (Actor|DestroyActor _array_element)))))