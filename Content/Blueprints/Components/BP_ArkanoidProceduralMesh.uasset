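; Procedural mesh component for the Arkanoid game that draws a flat, colored quad sized to a given box component.
; GenerateProceduralMesh builds one section from the box's X/Y extent at zero Z, writing the color into all vertices, then creates a dynamic instance of M_ProceduralMesh.
; ApplyBorder insets the quad by BorderSize as a fraction of the shorter side, keeping the margin uniform on both axes.
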(fn GenerateProceduralMesh
  (params (Box :type Box%20Component%20Object%20Reference) (Color :type Linear%20Color%20Structure))
  (LocalVariables|SetL_Box Box)
  (LocalVariables|SetL_Color Color)
  (LocalVariables|GetL_Box
    (:then
      (Class|ProceduralMeshComponent|CreateMeshSectionLinearColor 0 (Utilities|Array|MakeArray (Math|Vector|MakeVector (.X (Math|Vector|BreakVector (CallFunction|ApplyBorder (Variables|/Script/Engine.BoxComponent|GetBoxExtent (LocalVariables|GetL_Box))))) (* (.Y (Math|Vector|BreakVector (CallFunction|ApplyBorder (Variables|/Script/Engine.BoxComponent|GetBoxExtent (LocalVariables|GetL_Box))))) -1.0) 0.0) (Math|Vector|MakeVector (.X (Math|Vector|BreakVector (CallFunction|ApplyBorder (Variables|/Script/Engine.BoxComponent|GetBoxExtent (LocalVariables|GetL_Box))))) (.Y (Math|Vector|BreakVector (CallFunction|ApplyBorder (Variables|/Script/Engine.BoxComponent|GetBoxExtent (LocalVariables|GetL_Box))))) 0.0) (Math|Vector|MakeVector (* (.X (Math|Vector|BreakVector (CallFunction|ApplyBorder (Variables|/Script/Engine.BoxComponent|GetBoxExtent (LocalVariables|GetL_Box))))) -1.0) (.Y (Math|Vector|BreakVector (CallFunction|ApplyBorder (Variables|/Script/Engine.BoxComponent|GetBoxExtent (LocalVariables|GetL_Box))))) 0.0) (Math|Vector|MakeVector (* (.X (Math|Vector|BreakVector (CallFunction|ApplyBorder (Variables|/Script/Engine.BoxComponent|GetBoxExtent (LocalVariables|GetL_Box))))) -1.0) (* (.Y (Math|Vector|BreakVector (CallFunction|ApplyBorder (Variables|/Script/Engine.BoxComponent|GetBoxExtent (LocalVariables|GetL_Box))))) -1.0) 0.0)) (Utilities|Array|MakeArray 0 2 1 2 0 3) 0 (Utilities|Array|MakeArray "(X=0.000000,Y=0.000000)" "(X=1.000000,Y=0.000000)" "(X=1.000000,Y=1.000000)" "(X=0.000000,Y=1.000000)") 0 0 0 (Utilities|Array|MakeArray (LocalVariables|GetL_Color) (LocalVariables|GetL_Color) (LocalVariables|GetL_Color) (LocalVariables|GetL_Color)) 0 false)
      (Rendering|Material|CreateDynamicMaterialInstance 0 "/Game/Materials/M_ProceduralMesh.M_ProceduralMesh" "None" :!class /Script/Engine.PrimitiveComponent))
    (:else)))

(fn ApplyBorder
  (params (InSize :type Vector))
  (LocalVariables|SetL_Size InSize)
  (if (> (Variables|Settings|GetBorderSize) 0.0)
    (LocalVariables|SetL_Delta (* (.MinValue (Math|Float|MinOfFloatArray (Utilities|Array|MakeArray (.X (Math|Vector|BreakVector (LocalVariables|GetL_Size))) (.Y (Math|Vector|BreakVector (LocalVariables|GetL_Size)))))) (Variables|Settings|GetBorderSize)))
    (return (Math|Vector|MakeVector (- (.X (Math|Vector|BreakVector (LocalVariables|GetL_Size))) (LocalVariables|GetL_Delta)) (- (.Y (Math|Vector|BreakVector (LocalVariables|GetL_Size))) (LocalVariables|GetL_Delta)) (.Z (Math|Vector|BreakVector (LocalVariables|GetL_Size)))))
    (else
      (return (LocalVariables|GetL_Size)))))